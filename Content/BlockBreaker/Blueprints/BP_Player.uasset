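; BP_Player is the first-person player of BlockBreaker, handling movement, look and gun fire from axis inputs.
; On BeginPlay it spawns a BP_Rifle as EquippedGun and snaps it to GunLocation.
; Shooting passes a camera-forward trace segment to the gun's Shoot, with a CanShoot flag and Delay enforcing its FireRate.
; ChangeWeapon only returns a rifle or shotgun class, which the input event never uses to swap guns.
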(event EventBeginPlay
  ;[1 1 1] Choose weapon to attach
  (bind _returnvalue (Game|SpawnActorfromClass "/Game/BlockBreaker/Blueprints/BP_Rifle.BP_Rifle_C" (Math|Transform|MakeTransform "0, 0, 0" "0, 0, 0" "1,1,1") "Undefined" 0 0))
  (bind _output_get (Variables|Default|SetEquippedGun _returnvalue))
  (Transformation|AttachComponentToComponent _output_get (Variables|Default|GetGunLocation) "None" "SnapToTarget" "SnapToTarget" "KeepRelative" true))

(event Collision|EventActorBeginOverlap
  (params (OtherActor :type Actor%20Object%20Reference)))

(event EventTick
  (params (DeltaSeconds :type Float%20%28single-precision%29)))

(event Input|AxisEvents|InputAxisMoveForward
  (params (AxisValue :type Float%20%28single-precision%29))
  ;[1 1 1] Movement
  (Pawn|Input|AddMovementInput (Transformation|GetActorForwardVector) AxisValue false))

(event Input|AxisEvents|InputAxisMoveRight
  (params (AxisValue :type Float%20%28single-precision%29))
  ;[1 1 1] Movement
  (Pawn|Input|AddMovementInput (Transformation|GetActorRightVector) AxisValue false))

(event Input|AxisEvents|InputAxisLookHorizontal
  (params (AxisValue :type Float%20%28single-precision%29))
  ;[1 1 1] Camera
  (Pawn|Input|AddControllerYawInput AxisValue))

(event Input|AxisEvents|InputAxisLookVertical
  (params (AxisValue :type Float%20%28single-precision%29))
  ;[1 1 1] Camera
  (Pawn|Input|AddControllerPitchInput (* AxisValue -1.0)))

(event Input|AxisEvents|InputAxisShoot
  (params (AxisValue :type Float%20%28single-precision%29))
  (bind _fpscamera (Variables|Default|GetFpsCamera))
  (bind _returnvalue (Transformation|GetWorldLocation _fpscamera))
  ;[1 1 1] Shooting
  (if (and (== AxisValue 1.0) (Variables|Default|GetCanShoot))
    (Default|Shoot (Variables|Default|GetEquippedGun) _returnvalue (+ _returnvalue (* (Math|Vector|GetForwardVector _fpscamera) (Variables|/Game/BlockBreaker/Blueprints/BP_BaseGun.BP_BaseGun_C|GetMaxBulletDistance (Variables|Default|GetEquippedGun)))))
    (Variables|Default|SetCanShoot false)
    (Utilities|FlowControl|Delay (Variables|/Game/BlockBreaker/Blueprints/BP_BaseGun.BP_BaseGun_C|GetFireRate (Variables|Default|GetEquippedGun)))
    (Variables|Default|SetCanShoot true)))

(event Input|AxisEvents|InputAxisChangeWeapon
  (params (AxisValue :type Float%20%28single-precision%29))
  (CallFunction|ChangeWeapon AxisValue))

(fn ConstructionScript)

(fn ChangeWeapon
  (params (NewParam :type Float%20%28single-precision%29))
  (if (== NewParam 1.0)
    (bind _output_get (Variables|Default|SetRifle "/Game/BlockBreaker/Blueprints/BP_Rifle.BP_Rifle_C"))
    (return _output_get)
    (else
      (bind _output_get_2 (Variables|Default|SetShotgun "/Game/BlockBreaker/Blueprints/BP_Shotgun.BP_Shotgun_C"))
      (return _output_get_2))))