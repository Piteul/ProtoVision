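; BP_CGAPostProcess is an actor that configures a post process component to force a CGA palette look on the rendered scene.
; ApplySettings, run from the construction script, creates a dynamic material from one of two palette instances and sets its checker dither brightness from the screen dither strength.
; It also applies gamma, a color grading LUT indexed by palette and LUT dither level, and the enable toggle.
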(event Custom|ApplySettings
  (bind _gamma (Variables|Default|GetGamma))
  (bind _returnvalue (Rendering|Material|CreateDynamicMaterialInstance (select (Variables|Default|GetUse%20Palette%201) "/Game/CGAJam/PostProcessing/MI_ForceCGA_PP_Palette1.MI_ForceCGA_PP_Palette1" "/Game/CGAJam/PostProcessing/MI_ForceCGA_PP_Palette0.MI_ForceCGA_PP_Palette0") :!class /Script/Engine.KismetMaterialLibrary))
  (bind _output_get (Variables|Default|SetPostProcessMID _returnvalue))
  (Rendering|Material|SetScalarParameterValue _output_get "CheckerMinBrightness" (- 1.0 (Variables|Default|GetScreen%20Dither%20Strength)) :!class /Script/Engine.MaterialInstanceDynamic)
  (Utilities|Struct|SetmembersinPostProcessSettings (Variables|/Script/Engine.PostProcessComponent|GetSettings (Variables|Default|GetPostProcess)) (Math|Vector4|MakeVector4 _gamma _gamma _gamma _gamma) (Variables|Default|GetLUT%20Strength) (Utilities|Array|Get(acopy) (Variables|Default|GetLookupTextureList) (+ (Math|Integer|SelectInt 4 0 (Variables|Default|GetUse%20Palette%201)) (Variables|Default|GetLUT%20Dither%20Level))) (Utilities|Struct|MakeWeightedBlendables (Utilities|Array|MakeArray (Utilities|Struct|MakeWeightedBlendable 1.0 (Variables|Default|GetPostProcessMID)))))
  (Variables|/Script/Engine.PostProcessComponent|SetbEnabled (Variables|Default|GetPostProcess) (Variables|Default|GetEnable%20Postprocessing)))

(fn ConstructionScript
  (CallFunction|ApplySettings))